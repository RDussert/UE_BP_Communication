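; BP_Ennemy1 is a guard enemy that stays inactive until Activate turns LightsOn true, then patrols at random.
; Patrolling sets walk speed and chains AI moves to reachable points around its current location, repeating only on success.
; While lights are on, PawnSensing sightings set Spotted and start an AI move to the player with a printed shout.
; Reaching the player sets CanAttack, prints an attack line and applies fixed damage.
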(event `self.PawnSensing.OnSeePawn`
  (params (Pawn :type "Pawn Object Reference"))
  ;[1 1 1] Avant de déclencher les actions des ennemis on vérifie que la lumière est allumée
  (if (`self.LightsOn`)
    ;[1 1 1] Quand un ennemi repère le joueur il enclenche le script de poursuite
    (set `self.Spotted` true)
    (`self.FollowPlayer`)))

(event `FollowPlayer`
  (bind _returnvalue (`GameplayStatics.GetPlayerCharacter` 0))
  (bind _returnvalue_location (`KismetMathLibrary.BreakTransform` (`self.GetTransform` _returnvalue)))
  ;[1 1 1] Avant de déclencher les actions des ennemis on vérifie que la lumière est allumée
  (if (`self.Spotted`)
    ;[1 1 1] Quand un ennemi repère le joueur il crie HEY pour donner l'alerte et lancer la poursuite, si il arrive à porter du joueur il lui inflige 25  points de dégâts en disant TAKE THIS !
    (`KismetSystemLibrary.PrintString` "HEY !")
    (`|AIMoveTo` self _returnvalue_location _returnvalue
      (:`OnSuccess`
        (set `self.CanAttack` true)
        (`KismetSystemLibrary.PrintString` "TAKE THIS ! ")
        (`GameplayStatics.ApplyDamage` (`GameplayStatics.GetPlayerCharacter` 0) 25.0)))))

(event `PatrollingScript`
  ;[1 1 1] Avant de déclencher les actions des ennemis on vérifie que la lumière est allumée
  (if (`self.LightsOn`)
    ;[1 1 1] Quand un garde ne repère aucun intrus il patrouille sur la carte au hasard
    (set `CharacterMovementComponent.MaxWalkSpeed` (`self.Patrol Speed`) (`self.CharacterMovement`))
    (`|AIMoveTo` self (`NavigationSystemV1.K2_GetRandomReachablePointInRadius` (`self.K2_GetActorLocation`) (`self.Patrol Radius`) null null) null
      (:`OnSuccess`
        (`self.PatrollingScript`)))))

(event `/Game/Button/BPI_Interface.Activate`
  ;[1 1 1] Quand la lumière s'allume les gardes s'activent
  (set `self.LightsOn` true)
  (`self.PatrollingScript`))

(fn `UserConstructionScript`)