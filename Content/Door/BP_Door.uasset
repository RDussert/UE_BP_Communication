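; BP_Door is a door that toggles between open and closed when its Activate event fires, intended to come from a switch.
; Each toggle flips DoorOpen and runs the RotatingMovement component for a one-second Delay before deactivating it, with no direction change in the graph.
; Only the closing branch then calls Activate on Lights.
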(event `/Game/Button/BPI_Interface.Activate`
  (bind _rotatingmovement (`self.RotatingMovement`))
  ;[1 1 1] Quand on active un interrupteur on vérifie si les portes sont fermées ou ouvertes
  (if (`self.DoorOpen?`)
    ;[1 1 1] Si une portée est ouverte elle se ferme et le nombre de portes fermées augmente
    (set `self.DoorOpen?` false)
    (`ActorComponent.Activate` _rotatingmovement false)
    (`KismetSystemLibrary.Delay` 1.0)
    (`ActorComponent.Deactivate` _rotatingmovement)
    (`/Game/Button/BPI_Interface.Activate` (`self.Lights`))
    (else
      ;[1 1 1] Si une porte est fermée elle s'ouvre
      (set `self.DoorOpen?` true)
      (`ActorComponent.Activate` (`self.RotatingMovement`) false)
      (`KismetSystemLibrary.Delay` 1.0)
      (`ActorComponent.Deactivate` (`self.RotatingMovement`)))))

(fn `UserConstructionScript`)